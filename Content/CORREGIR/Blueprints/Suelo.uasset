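; Suelo is a floor actor that, on its OpenFloor event, shrinks away along the X axis and then destroys itself.
; It saves the original transform, then lerps the world scale of the Rr component toward an X scale reduced by 30.
; A Delay of one frame's delta seconds loops the update like a Tick, advancing by Speed until done, then prints "Loos" before DestroyActor.
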(event `OpenFloor`
  (bind _original_scale (`self.original scale`))
  ;[1 1 1] Guardar Scala original
  (set `self.original scale` (`self.GetTransform`))
  ;[1 1 1] Posicion final
  (bind _output_get (set `self.rescalado` (`KismetMathLibrary.MakeTransform` (.location _original_scale) (.rotation _original_scale) (`KismetMathLibrary.MakeVector` (- (.x (.scale _original_scale)) 30.0) (.y (.scale _original_scale)) (.z (.scale _original_scale))))))
  ;[1 1 1] Setear el Aloha para el lerp
  (bind _output_get_2 (set `self.time ` (+ (* (`self.speed`) (`GameplayStatics.GetWorldDeltaSeconds`)) (`self.time `)) :!label _label))
  (bind (_returnvalue_location _returnvalue_rotation _returnvalue_scale) (`KismetMathLibrary.BreakTransform` (`KismetMathLibrary.TLerp` (`self.original scale`) (`KismetMathLibrary.MakeTransform` (.location _output_get) (.rotation _output_get) (.scale _output_get)) _output_get_2)))
  ;[1 1 1] seteadole el lerp al la word Scale
  (`SceneComponent.SetWorldScale3D` (`self.rr`) _returnvalue_scale)
  ;[1 1 1] Delay par simular el event tick
  (`KismetSystemLibrary.Delay` (`GameplayStatics.GetWorldDeltaSeconds`))
  ;[1 1 1] Comprobos si ya llegado a su posicion final
  (if (>= (`self.time `) 1.0)
    ;[1 1 1] Cuado acabe el bucle printa un text y destrulle el Actor
    (`KismetSystemLibrary.PrintText` "Loos" true true (struct :`R` 1.0 :`G` 0.076844 :`A` 1.0))
    (`self.K2_DestroyActor`)
    (else
      (goto _label))))

(fn `UserConstructionScript`)