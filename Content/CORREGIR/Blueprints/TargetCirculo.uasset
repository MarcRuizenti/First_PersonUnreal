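; TargetCirculo is a moving shooting target that awards score when hit by a first-person projectile.
; BeginPlay sets its speed, and Tick moves it with sweep along the right vector of its Arrow component.
; When Sphere1 is hit by a BP_FirstPersonProjectile, it calls SumeScore on the GameManager found in the level, then destroys itself and the projectile.
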(event `self.ReceiveBeginPlay`
  (set `self.Velocidad` 300.0))

(event `self.ReceiveTick`
  (params (DeltaSeconds :type "Float (single-precision)"))
  (`self.K2_AddActorWorldOffset` (* (* DeltaSeconds (`self.Velocidad`)) (`SceneComponent.GetRightVector` (`self.Arrow`))) true))

(event `self.Sphere1.OnComponentHit`
  (params (HitComponent :type "PrimitiveComponent Object Reference") (OtherActor :type "Actor Object Reference") (OtherComp :type "PrimitiveComponent Object Reference") (NormalImpulse :type "Vector Structure") (Hit :type "HitResult Structure (by ref)"))
  (bind _asbp_first_person_projectile (cast `/Game/FirstPerson/Blueprints/BP_FirstPersonProjectile` OtherActor))
  (bind _returnvalue (`GameplayStatics.GetActorOfClass` "/Game/CORREGIR/Blueprints/GameManager.GameManager_C"))
  (`/Game/CORREGIR/Blueprints/GameManager.SumeScore` _returnvalue)
  (`self.K2_DestroyActor`)
  (`self.K2_DestroyActor` _asbp_first_person_projectile))

(fn `UserConstructionScript`)