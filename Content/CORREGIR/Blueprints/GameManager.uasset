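; GameManager Blueprint that runs a printed start countdown and then starts the game through TManager.
; BeginPlay clears the Start flag and resets CuentaAtras, and Tick waits for Start to become true.
; The Contador macro clears Start so it triggers once, then loops through a one-second Delay, decrementing and printing the count.
; At zero it prints START and exits, calling StartGame on TManager.
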(event `self.ReceiveBeginPlay`
  (set `self.Start` false)
  (set `self.CuentaAtras` 5))

(event `self.ReceiveTick`
  (params (DeltaSeconds :type "Float (single-precision)"))
  (if (`self.Start`)
    (`self.Contador`
      (:`exit`
        (`/Game/CORREGIR/Blueprints/TargetManager.Start Game` (`self.TManager`))))))

(fn `UserConstructionScript`)