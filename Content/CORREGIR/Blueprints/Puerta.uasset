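; Puerta is a door Blueprint that swings its Door component 90 degrees in yaw when the OpenDoor event is called.
; OpenDoor stores the initial world rotation and lerps toward the target, with an alpha that grows by Speed times delta seconds.
; A looping Delay of one frame's delta stands in for Tick until the alpha reaches 1, then it prints "open".
; Time is never reset, and there is no closing logic.
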(event `OpenDoor`
  (bind (_rtacion_inicial_roll _rtacion_inicial_pitch _rtacion_inicial_yaw) (`KismetMathLibrary.BreakRotator` (`self.rtacion inicial`)))
  ;[1 1 1] Guardando rotacion inicial
  (set `self.rtacion inicial` (`SceneComponent.K2_GetComponentRotation` (`self.door`)))
  ;[1 1 1] Seteando el alpha para el lerp
  (bind _output_get (set `self.time` (+ (`self.time`) (* (`self.speed`) (`GameplayStatics.GetWorldDeltaSeconds`))) :!label _label))
  ;[1 1 1] Seteando la nueva rotacion
  (bind _output_get_2 (set `self.rotation` (`KismetMathLibrary.MakeRotator` _rtacion_inicial_roll _rtacion_inicial_pitch (+ _rtacion_inicial_yaw 90.0))))
  ;[1 1 1] Seteando le a la World rotation el lerp
  (`SceneComponent.K2_SetWorldRotation` (`self.door`) (`KismetMathLibrary.RLerp` (`self.rtacion inicial`) _output_get_2 _output_get) false false)
  ;[1 1 1] simulando el event tick
  (`KismetSystemLibrary.Delay` (`GameplayStatics.GetWorldDeltaSeconds`))
  ;[1 1 1] Comprovamos a acabado el movimiento
  (if (>= (`self.time`) 1.0)
    (`KismetSystemLibrary.PrintText` "open")
    (else
      (goto _label))))

(fn `UserConstructionScript`)