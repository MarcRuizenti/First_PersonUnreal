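; TargetManager spawns a random target at each of its target points when the game starts.
; The StartGame event loops over the TPoints array and calls SpawnTargets for every point.
; SpawnTargets picks a random integer to spawn a cone, circle or cube target class at that point's location and rotation.
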(event `Start Game`
  ;[1 1 1] Hacemos un bucle para spawnar targets en todos los target points
  (for _array_element (`self.TPoints`)
    (`self.SpawnTargets` _array_element)))

(fn `UserConstructionScript`)